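; Security camera actor that a player pans and tilts while interacting, linked through a SecurityMonitor_BP.
; RotateCamera applies sensitivity-scaled input to KameraMonitor's relative pitch and yaw, clamped to configurable limits.
; Tick caches the world rotation of the monitor's current camera during interaction.
; The W/A/S/D events compare it against hard-coded limits to start or stop the rotation sound, using per-direction Stop flags that ResetSFX re-enables.
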(event `self.ReceiveBeginPlay`
  (bind _returnvalue (`GameplayStatics.GetActorOfClass` "/Game/Camera_System/SecurityMonitor_BP.SecurityMonitor_BP_C"))
  (bind _returnvalue_2 (`GameplayStatics.GetActorOfClass` "/Game/ThirdPerson/Blueprints/BP_ThirdPersonCharacter.BP_ThirdPersonCharacter_C"))
  (set `self.İnteract On TP_BP` _returnvalue_2))

(event `self.ReceiveTick`
  (params (DeltaSeconds :type "Float (single-precision)"))
  (if (`/Game/ThirdPerson/Blueprints/BP_ThirdPersonCharacter.IsInteracting` (`self.İnteract On TP_BP`))
    (set `self.Y (Pitch)` (.pitch (`SceneComponent.K2_GetComponentRotation` (`/Game/Camera_System/SecurityCamera_BP.KameraMonitor` (`|GetArrayItem` (`/Game/Camera_System/SecurityMonitor_BP.LinkedCameras` (stale `self.ReceiveBeginPlay` _returnvalue)) (`/Game/Camera_System/SecurityMonitor_BP.CurrentCamera` (stale `self.ReceiveBeginPlay` _returnvalue)))))))
    (set `self.Z (Yaw)` (.yaw (`SceneComponent.K2_GetComponentRotation` (`/Game/Camera_System/SecurityCamera_BP.KameraMonitor` (`|GetArrayItem` (`/Game/Camera_System/SecurityMonitor_BP.LinkedCameras` (stale `self.ReceiveBeginPlay` _returnvalue)) (`/Game/Camera_System/SecurityMonitor_BP.CurrentCamera` (stale `self.ReceiveBeginPlay` _returnvalue)))))))))

(event `Rotate Cam W`
  (bind _i_nteract_on_tp_bp (`self.İnteract On TP_BP`))
  (bind _rotatecamera_sfx (`self.RotateCamera_SFX`))
  (bind _pressed_released (`/Game/ThirdPerson/Blueprints/BP_ThirdPersonCharacter.Pressed/Released` (`self.İnteract On TP_BP`)))
  (if (`self.Stop W`)
    (if (`/Game/ThirdPerson/Blueprints/BP_ThirdPersonCharacter.IsInteracting` _i_nteract_on_tp_bp)
      (if (`/Game/ThirdPerson/Blueprints/BP_ThirdPersonCharacter.Pressed/Released` _i_nteract_on_tp_bp)
        (if (< (`self.Y (Pitch)`) 15.0)
          (`ActorComponent.Activate` _rotatecamera_sfx false)
          (if _pressed_released
            (set `self.Stop S` true))
          (else
            (`AudioComponent.Stop` _rotatecamera_sfx :!label _label)
            (if _pressed_released
              (set `self.Stop W` false))))
        (else
          (goto _label)))
      (else
        (goto _label)))))

(event `Rotate Cam S`
  (bind _i_nteract_on_tp_bp (`self.İnteract On TP_BP`))
  (bind _rotatecamera_sfx (`self.RotateCamera_SFX`))
  (bind _pressed_released (`/Game/ThirdPerson/Blueprints/BP_ThirdPersonCharacter.Pressed/Released` (`self.İnteract On TP_BP`)))
  (if (`self.Stop S`)
    (if (`/Game/ThirdPerson/Blueprints/BP_ThirdPersonCharacter.IsInteracting` _i_nteract_on_tp_bp)
      (if (`/Game/ThirdPerson/Blueprints/BP_ThirdPersonCharacter.Pressed/Released` _i_nteract_on_tp_bp)
        (if (> (`self.Y (Pitch)`) -45.0)
          (`ActorComponent.Activate` _rotatecamera_sfx false)
          (if _pressed_released
            (set `self.Stop W` true))
          (else
            (`AudioComponent.Stop` _rotatecamera_sfx :!label _label_2)
            (if _pressed_released
              (set `self.Stop S` false))))
        (else
          (goto _label_2)))
      (else
        (goto _label_2)))))

(event `Rotate Cam D`
  (bind _i_nteract_on_tp_bp (`self.İnteract On TP_BP`))
  (bind _rotatecamera_sfx (`self.RotateCamera_SFX`))
  (bind _pressed_released (`/Game/ThirdPerson/Blueprints/BP_ThirdPersonCharacter.Pressed/Released` (`self.İnteract On TP_BP`)))
  (if (`self.Stop D`)
    (if (`/Game/ThirdPerson/Blueprints/BP_ThirdPersonCharacter.IsInteracting` _i_nteract_on_tp_bp)
      (if (`/Game/ThirdPerson/Blueprints/BP_ThirdPersonCharacter.Pressed/Released` _i_nteract_on_tp_bp)
        (if (< (`self.Z (Yaw)`) 45.0)
          (`ActorComponent.Activate` _rotatecamera_sfx false)
          (if _pressed_released
            (set `self.Stop A` true))
          (else
            (`AudioComponent.Stop` _rotatecamera_sfx :!label _label_3)
            (if _pressed_released
              (set `self.Stop D` false))))
        (else
          (goto _label_3)))
      (else
        (goto _label_3)))))

(event `Rotate Cam A`
  (bind _i_nteract_on_tp_bp (`self.İnteract On TP_BP`))
  (bind _rotatecamera_sfx (`self.RotateCamera_SFX`))
  (bind _pressed_released (`/Game/ThirdPerson/Blueprints/BP_ThirdPersonCharacter.Pressed/Released` (`self.İnteract On TP_BP`)))
  (if (`self.Stop A`)
    (if (`/Game/ThirdPerson/Blueprints/BP_ThirdPersonCharacter.IsInteracting` _i_nteract_on_tp_bp)
      (if (`/Game/ThirdPerson/Blueprints/BP_ThirdPersonCharacter.Pressed/Released` _i_nteract_on_tp_bp)
        (if (> (`self.Z (Yaw)`) -45.0)
          (`ActorComponent.Activate` _rotatecamera_sfx false)
          (if _pressed_released
            (set `self.Stop D` true))
          (else
            (`AudioComponent.Stop` _rotatecamera_sfx :!label _label_4)
            (if _pressed_released
              (set `self.Stop A` false))))
        (else
          (goto _label_4)))
      (else
        (goto _label_4)))))

(event `Reset SFX`
  (set `self.Stop W` true)
  (set `self.Stop A` true)
  (set `self.Stop S` true)
  (set `self.Stop D` true))

(fn `RotateCamera`
  (params (HorizontalShift :type "Float (double-precision)") (VerticalShift :type "Float (double-precision)"))
  (bind (_relativerotation_roll _relativerotation_pitch _relativerotation_yaw) (`KismetMathLibrary.BreakRotator` (`SceneComponent.RelativeRotation` (`self.KameraMonitor`))))
  (`SceneComponent.K2_SetRelativeRotation` (`self.KameraMonitor`) (`KismetMathLibrary.MakeRotator` 0.0 (`KismetMathLibrary.FClamp` (+ _relativerotation_pitch (* (`local.VerticalShift`) (`self.VerticalSensitivity`))) (`self.MaxDownRotation`) (`self.MaxUpRotation`)) (`KismetMathLibrary.FClamp` (+ _relativerotation_yaw (* (`local.HorizontalShift`) (`self.HorizontalSensitivity`))) (`self.MaxLeftRotation`) (`self.MaxRightRotation`))) false false))

(fn `UserConstructionScript`)