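; Security monitor actor that shows live feeds from linked security cameras and forwards player input to rotate the active one.
; Each camera's scene capture feeds a viewport-scaled render target on the screen's dynamic material, recreated on every swap.
; A delayed Tick captures continuously while the player is interacting, otherwise takes periodic snapshots to save cost.
; Swapping cycles through linked cameras, though backward wraparound uses a hardcoded last index.
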(event `self.ReceiveTick`
  (params (DeltaSeconds :type "Float (single-precision)"))
  (bind _kameramonitor (`/Game/Camera_System/SecurityCamera_BP.KameraMonitor` (`|GetArrayItem` (`self.LinkedCameras`) (`self.CurrentCamera`))))
  (set `self.CurrentCamera` (`self.CurrentCamera`))
  (`KismetSystemLibrary.Delay` 0.2)
  (if (`/Game/ThirdPerson/Blueprints/BP_ThirdPersonCharacter.IsInteracting` (`self.TP Character REF`))
    (set `SceneCaptureComponent.bCaptureOnMovement` true _kameramonitor)
    (set `SceneCaptureComponent.bCaptureEveryFrame` (`SceneCaptureComponent.bCaptureOnMovement` _kameramonitor) _kameramonitor)
    (else
      (`SceneCaptureComponent2D.CaptureScene` _kameramonitor)
      (set `SceneCaptureComponent.bCaptureOnMovement` false _kameramonitor)
      (set `SceneCaptureComponent.bCaptureEveryFrame` false _kameramonitor))))

(event `self.ReceiveBeginPlay`
  (bind (_returnvalue_x _returnvalue_y) (`KismetMathLibrary.BreakVector2D` (`WidgetLayoutLibrary.GetViewportSize`)))
  (bind _cameraqualitylevel (`/Game/Camera_System/SecurityCamera_BP.CameraQualityLevel` (`|GetArrayItem` (`self.LinkedCameras`))))
  (bind _returnvalue (`GameplayStatics.GetActorOfClass` "/Game/ThirdPerson/Blueprints/BP_ThirdPersonCharacter.BP_ThirdPersonCharacter_C"))
  (set `self.TP Character REF` _returnvalue)
  (bind _outactors (`GameplayStatics.GetAllActorsOfClass` "/Game/Camera_System/SecurityCamera_BP.SecurityCamera_BP_C"))
  (set `self.Active Camera ACT` _outactors)
  (`/Engine/EditorBlueprintResources/StandardMacros.IsValid` (`|GetArrayItem` (`self.LinkedCameras`))
    (:`Is Valid`
      (bind _returnvalue_2 (`KismetMaterialLibrary.CreateDynamicMaterialInstance` "/Game/Camera_System/Materials/SC_Mat.SC_Mat"))
      (bind _output_get (set `self.Camera_MAT` _returnvalue_2))
      (`PrimitiveComponent.SetMaterial` (`self.Monitor`) 0 _output_get)
      (bind _returnvalue_3 (`KismetRenderingLibrary.CreateRenderTarget2D` (`KismetMathLibrary.FTrunc` (* _returnvalue_x _cameraqualitylevel)) (`KismetMathLibrary.FTrunc` (* _returnvalue_y _cameraqualitylevel))))
      (bind _output_get_2 (set `self.Camera_RT` _returnvalue_3))
      (bind _output_get_3 (set `SceneCaptureComponent2D.TextureTarget` _output_get_2 (`/Game/Camera_System/SecurityCamera_BP.KameraMonitor` (`|GetArrayItem` (`self.LinkedCameras`)))))
      (`MaterialInstanceDynamic.SetTextureParameterValue` (`self.Camera_MAT`) "Texture" _output_get_3)
      (`MaterialInstanceDynamic.SetScalarParameterValue` (`self.Camera_MAT`) "ScreenBrightness" (`self.ScreenBrightness`)))))

(event `NewPlayerInput`
  (params (HorizontalValue :type "Float (double-precision)") (VerticalValue :type "Float (double-precision)"))
  (`/Game/Camera_System/SecurityCamera_BP.RotateCamera` (`|GetArrayItem` (`self.LinkedCameras`) (`self.CurrentCamera`)) HorizontalValue VerticalValue))

(event `SwapCamera`
  (bind (_returnvalue_x _returnvalue_y) (`KismetMathLibrary.BreakVector2D` (`WidgetLayoutLibrary.GetViewportSize`)))
  (bind _currentcamera (`self.CurrentCamera`))
  (bind _cameraqualitylevel (`/Game/Camera_System/SecurityCamera_BP.CameraQualityLevel` (`|GetArrayItem` (`self.LinkedCameras`) (`self.CurrentCamera`))))
  (set `SceneCaptureComponent2D.TextureTarget` null (`/Game/Camera_System/SecurityCamera_BP.KameraMonitor` (`|GetArrayItem` (`self.LinkedCameras`) (`self.CurrentCamera`))))
  (`/Engine/EditorBlueprintResources/StandardMacros.IncrementInt` _currentcamera
    (:`  `
      (if (>= _currentcamera (`KismetArrayLibrary.Array_Length` (`self.LinkedCameras`)))
        (set `self.CurrentCamera` 0))
      (bind _returnvalue (`KismetRenderingLibrary.CreateRenderTarget2D` (`KismetMathLibrary.FTrunc` (* _returnvalue_x _cameraqualitylevel)) (`KismetMathLibrary.FTrunc` (* _returnvalue_y _cameraqualitylevel))))
      (bind _output_get (set `self.Camera_RT` _returnvalue))
      (bind _output_get_2 (set `SceneCaptureComponent2D.TextureTarget` _output_get (`/Game/Camera_System/SecurityCamera_BP.KameraMonitor` (`|GetArrayItem` (`self.LinkedCameras`) (`self.CurrentCamera`)))))
      (`MaterialInstanceDynamic.SetTextureParameterValue` (`self.Camera_MAT`) "Texture" _output_get_2))))

(event `SwapCameraBack`
  (bind (_returnvalue_x _returnvalue_y) (`KismetMathLibrary.BreakVector2D` (`WidgetLayoutLibrary.GetViewportSize`)))
  (bind _currentcamera (`self.CurrentCamera`))
  (bind _cameraqualitylevel (`/Game/Camera_System/SecurityCamera_BP.CameraQualityLevel` (`|GetArrayItem` (`self.LinkedCameras`) (`self.CurrentCamera`))))
  (set `SceneCaptureComponent2D.TextureTarget` null (`/Game/Camera_System/SecurityCamera_BP.KameraMonitor` (`|GetArrayItem` (`self.LinkedCameras`) (`self.CurrentCamera`))))
  (`/Engine/EditorBlueprintResources/StandardMacros.DecrementInt` _currentcamera
    (:`  `
      (if (<= 0 _currentcamera)
        _
        (elif (<= 0 (`KismetArrayLibrary.Array_Length` (`self.LinkedCameras`)))
          ;[1 1 1] Sec-Mon Bp En büyük Kamera değerini buraya yaz.
          (set `self.CurrentCamera` 3)))
      (bind _returnvalue (`KismetRenderingLibrary.CreateRenderTarget2D` (`KismetMathLibrary.FTrunc` (* _returnvalue_x _cameraqualitylevel)) (`KismetMathLibrary.FTrunc` (* _returnvalue_y _cameraqualitylevel))))
      (bind _output_get (set `self.Camera_RT` _returnvalue))
      (bind _output_get_2 (set `SceneCaptureComponent2D.TextureTarget` _output_get (`/Game/Camera_System/SecurityCamera_BP.KameraMonitor` (`|GetArrayItem` (`self.LinkedCameras`) (`self.CurrentCamera`)))))
      (`MaterialInstanceDynamic.SetTextureParameterValue` (`self.Camera_MAT`) "Texture" _output_get_2))))

(fn `UserConstructionScript`)