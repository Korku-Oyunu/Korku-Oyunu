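; Light switch actor that lets the player toggle linked Light_BP lights with the F key.
; Box overlap shows a prompt widget, enables input and opens a gate so the key works only in range.
; BeginPlay caches all Light_BP actors, and a press toggles those sharing the switch's LightIndex.
; Each toggle activates a switch effect and plays or reverses a timeline that tilts the switch based on IsOn.
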(event `Key|F`
  (params (Key :type "Key Structure"))
  (:`Pressed`
    (`/Engine/EditorBlueprintResources/StandardMacros.Gate` true :!label _label
      (:`Exit`
        (for _array_element (`self.Lights Array`)
          (if (== (`/Game/LevelDesign/LightningSystem/Light_BP.LightIndex` _array_element) (`self.Light Index`))
            (message `/Game/Interfaces/Interaction.Toggle Lights` _array_element)
            (`ActorComponent.Activate` (`self.LightSwitchEffect`) true)
            (if (`/Game/LevelDesign/LightningSystem/Light_BP.IsOn?` (stale `self.ReceiveBeginPlay` _array_element))
              (bind (_direction _lightswitchalpha) (`Timeline|Lightwitch_TL` :!label _label_2)
                (:`Update`
                  (`SceneComponent.K2_SetRelativeRotation` (`self.Switch`) (`KismetMathLibrary.MakeRotator` 0.0 (`KismetMathLibrary.Lerp` 0.0 -10.0 _lightswitchalpha)) false false)))
              (else
                (goto _label_2 :!via `Reverse`)))))))))

(event `self.Box.OnComponentBeginOverlap`
  (params (OverlappedComponent :type "PrimitiveComponent Object Reference") (OtherActor :type "Actor Object Reference") (OtherComp :type "PrimitiveComponent Object Reference") (OtherBodyIndex :type Integer) (bFromSweep :type Boolean) (SweepResult :type "HitResult Structure (by ref)"))
  (`SceneComponent.SetVisibility` (`self.Widget`) true false)
  (`self.EnableInput` (`GameplayStatics.GetPlayerController` 0))
  (goto _label :!via `Open`))

(event `self.Box.OnComponentEndOverlap`
  (params (OverlappedComponent :type "PrimitiveComponent Object Reference") (OtherActor :type "Actor Object Reference") (OtherComp :type "PrimitiveComponent Object Reference") (OtherBodyIndex :type Integer))
  (`SceneComponent.SetVisibility` (`self.Widget`) false false)
  (`self.DisableInput` (`GameplayStatics.GetPlayerController` 0))
  (goto _label :!via `Close`))

(event `self.ReceiveBeginPlay`
  (bind _outactors (`GameplayStatics.GetAllActorsOfClass` "/Game/LevelDesign/LightningSystem/Light_BP.Light_BP_C"))
  (for _array_element _outactors
    (`KismetArrayLibrary.Array_Add` (`self.Lights Array`) _array_element)))

(fn `UserConstructionScript`)