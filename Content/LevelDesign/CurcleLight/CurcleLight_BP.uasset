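; Circle lamp Blueprint that switches between on, off and flickering looks by swapping the lamp material.
; The construction script applies the on or off material from IsOn, and ToggleLights inverts that flag at runtime, updating MaterialIsOn alongside it.
; Flicker uses a FlipFlop to alternate between the flicker material with its ambiance component active and the steady on material with it stopped, regardless of IsOn.
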(event `Flicker`
  (bind _flickerlights_ambiance1 (`self.FlickerLights_Ambiance1`))
  (bind _lamp (`self.Lamp`))
  (`/Engine/EditorBlueprintResources/StandardMacros.FlipFlop`
    (:`A`
      (`PrimitiveComponent.SetMaterial` _lamp 0 "/Game/LevelDesign/CurcleLight/LampFlicker.LampFlicker")
      (`ActorComponent.Activate` _flickerlights_ambiance1 false))
    (:`B`
      (`PrimitiveComponent.SetMaterial` _lamp 0 "/Game/LevelDesign/CurcleLight/MI_Lamp1On.MI_Lamp1On")
      (`AudioComponent.Stop` _flickerlights_ambiance1))))

(event `self.Toggle Lights`
  (bind _lamp (`self.Lamp`))
  (set `self.IsOn?` (not (`self.IsOn?`)))
  (if (`self.IsOn?`)
    (set `self.MaterialIsOn?` true)
    (`PrimitiveComponent.SetMaterial` _lamp 0 "/Game/LevelDesign/CurcleLight/MI_Lamp1On.MI_Lamp1On")
    (else
      (set `self.MaterialIsOn?` false)
      (`PrimitiveComponent.SetMaterial` _lamp 0 "/Game/ScienceLab/Materials/Rooms/MI_Lamp.MI_Lamp"))))

(fn `UserConstructionScript`
  (bind _lamp (`self.Lamp`))
  (bind _materialison_ (`self.MaterialIsOn?`))
  (if (`self.IsOn?`)
    (set `self.MaterialIsOn?` _materialison_)
    (`PrimitiveComponent.SetMaterial` _lamp 0 "/Game/LevelDesign/CurcleLight/MI_Lamp1On.MI_Lamp1On")
    (else
      (set `self.MaterialIsOn?` _materialison_)
      (`PrimitiveComponent.SetMaterial` _lamp 0 "/Game/ScienceLab/Materials/Rooms/MI_Lamp.MI_Lamp"))))